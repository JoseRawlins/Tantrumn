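; EpicCharacter is a character Blueprint that prints jump diagnostics for tuning movement.
; OnJumped stores the start position and prints velocity, and OnLanded prints the distance travelled.
; Apex and jump time helpers are not called here, and the node setting their start time is unwired.
; A Hold macro separates Tap from Held input using a retriggerable delay and two gates.
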(event `self.OnJumped`
  (set `self.StartPosition` (`self.K2_GetActorLocation`))
  (`KismetSystemLibrary.PrintString` (`KismetStringLibrary.Conv_VectorToString` (`self.GetVelocity`))))

(event `self.OnLanded`
  (params (Hit :type "HitResult Structure (by ref)"))
  (`KismetSystemLibrary.PrintString` "JumpDistance:" true true (struct :`G` 0.66 :`B` 1.0 :`A` 1.0) 5.0)
  (`KismetSystemLibrary.PrintString` (`KismetStringLibrary.Conv_DoubleToString` (`KismetMathLibrary.VSize` (- (`self.K2_GetActorLocation`) (`self.StartPosition`)))) true true (struct :`G` 0.66 :`B` 1.0 :`A` 1.0) 5.0))

(event `self.ReceiveTick`
  (params (DeltaSeconds :type "Float (single-precision)")))

(fn `PrintApexTime`
  (bind (_returnvalue_x _returnvalue_y _returnvalue_z) (`KismetMathLibrary.BreakVector` (`self.GetVelocity`)))
  (bind (_lastvelocity_x _lastvelocity_y _lastvelocity_z) (`KismetMathLibrary.BreakVector` (`self.LastVelocity`)))
  (if (and (> _lastvelocity_z 0.0) (< _returnvalue_z 0.0))
    (`KismetSystemLibrary.PrintString` "ApexTime:" true true (struct :`R` 0.963968 :`G` 1.0 :`A` 1.0) 10.0)
    (`KismetSystemLibrary.PrintString` (`KismetStringLibrary.Conv_DoubleToString` (- (`GameplayStatics.GetTimeSeconds`) (`self.JumpStartTime`))) true true (struct :`R` 0.120293 :`G` 1.0 :`A` 1.0) 10.0))
  (set `self.LastVelocity` (`self.GetVelocity`)))

(fn `PrintJumpTime`
  (`KismetSystemLibrary.PrintString` "JumpTime:" true true (struct :`G` 0.66 :`B` 1.0 :`A` 1.0) 10.0)
  (`KismetSystemLibrary.PrintString` (`KismetStringLibrary.Conv_DoubleToString` (- (`GameplayStatics.GetTimeSeconds`) (`self.JumpStartTime`))) true true (struct :`G` 0.66 :`B` 1.0 :`A` 1.0) 10.0))

(fn `UserConstructionScript`)